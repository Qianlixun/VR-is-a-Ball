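; VR pawn for a rolling-ball game, steered with motion controllers, with start and pause menus and a gold score counter.
; Each Tick aims an arrow at twice the right controller's yaw and applies torque from the arrow's heading, signed forward or back by the right or left button.
; Spawned widget actors serve as menus; while paused, the left button becomes a widget-interaction mouse click.
; Keyboard and camera-rotation branches are unwired.
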(event EventTick
  (params (DeltaSeconds :type Float%20%28single-precision%29))
  ;[1 1 1] 球产生滚动
  (Utilities|FlowControl|Sequence
    (:then_0
      (Class|PrimitiveComponent|AddTorque (Variables|Default|GetBall) (* (* (Math|Vector|GetRightVector (Math|Rotator|MakeRotator 0.0 0.0 (* 2 (.Yaw (Math|Rotator|BreakRotator (Transformation|GetSocketRotation (Variables|Default|GetArrow) "None")))))) (Variables|Default|GetRunSpeed)) (Variables|Default|GetForB)) "None" false))
    (:then_1
      (Transformation|SetWorldRotation (Variables|Default|GetArrow) (Math|Rotator|MakeRotator 0.0 0.0 (* 2 (.Yaw (Math|Rotator|BreakRotator (Transformation|GetWorldRotation (Variables|Default|GetRightMotionController)))))) false false))))

(event EventBeginPlay
  ;[1 1 1] 创建开始菜单
  (bind _returnvalue (Game|SpawnActorfromClass "/Game/BluePrint/dgz/Begin_widge.Begin_widge_C" (Transformation|GetWorldTransform (Variables|Default|GetWidgeLocation)) "AlwaysSpawn" 0 0))
  (Variables|Default|SetBeginWidge _returnvalue)
  (Variables|Default|SetIsPause true)
  (Variables|Default|SetCanWalk false)
  (Variables|Default|SetCanPause false))

(event Input|ActionEvents|InputActionGameStop
  (params (Key :type Key%20Structure :default "AnyKey"))
  ;[1 1 1] 创建暂停菜单
  (:Pressed
    (if (Variables|Default|GetCanPause)
      (if (not (Variables|Default|GetIsPause))
        (bind _returnvalue (Game|SpawnActorfromClass "/Game/BluePrint/dgz/Stop_widge.Stop_widge_C" (Transformation|GetWorldTransform (Variables|Default|GetWidgeLocation)) "AlwaysSpawn" 0 0))
        (bind _output_get (Variables|Default|SetWidgeActor _returnvalue))
        (Class|ActorComponent|SetTickablewhenPaused (Variables|/Game/BluePrint/dgz/Stop_widge.Stop_widge_C|GetWidget _output_get) true)
        (Class|ActorComponent|SetTickablewhenPaused (Variables|Default|GetBall) false)
        (Game|SetGamePaused true)
        (Variables|Default|SetIsPause true)
        (Variables|Default|SetCanPause false)
        (Variables|Default|SetCanWalk false)))))

(event Input|ActionEvents|InputActionLeftMotionTaked
  (params (Key :type Key%20Structure :default "AnyKey"))
  (bind _widgetinteraction (Variables|Default|GetWidgetInteraction))
  (bind _ispause (Variables|Default|GetIsPause))
  (:Pressed
    (if _ispause
      ;[1 1 1] 暂停后手柄代替鼠标左键
      (Class|WidgetInteractionComponent|PressPointerKey _widgetinteraction "LeftMouseButton")
      (else
        (Variables|Default|SetMotionFire true)
        (Variables|Default|SetForB -1))))
  (:Released
    (if _ispause
      (Class|WidgetInteractionComponent|ReleasePointerKey _widgetinteraction "LeftMouseButton")
      (else
        (Variables|Default|SetMotionFire false)
        (Variables|Default|SetForB 0)))))

(event Input|ActionEvents|InputActionRightMotionTaked
  (params (Key :type Key%20Structure :default "AnyKey"))
  (bind _ispause (Variables|Default|GetIsPause))
  (:Pressed
    (if (not _ispause)
      (Variables|Default|SetMotionFire true)
      (Variables|Default|SetForB 1)))
  (:Released
    (if (not _ispause)
      (Variables|Default|SetMotionFire false)
      (Variables|Default|SetForB 0))))

(fn ConstructionScript)

(fn ResumeMyGame
  (bind _widgeactor (Variables|Default|GetWidgeActor))
  (Variables|Default|SetIsPause false)
  (Utilities|IsValid _widgeactor
    (:Is%20Valid
      (Actor|DestroyActor _widgeactor)
      (Game|SetGamePaused false))))

(fn DeleteBeginWidge
  (Actor|DestroyActor)
  (Variables|Default|SetCanWalk true))

(fn AddScore
  (Variables|Default|SetGold (+ (Variables|Default|GetGold) 1)))