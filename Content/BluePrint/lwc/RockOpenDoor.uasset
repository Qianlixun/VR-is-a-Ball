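; RockOpenDoor is a two-panel rock door that opens when something overlaps its Box trigger and closes when the overlap ends.
; The RockMovement timeline plays or reverses, lerping StaticMesh and StaticMesh1 apart along Y between hard-coded world positions, so the door is tied to one level location.
; Both overlap events play the same 2D sound and do not filter the overlapping actor.
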(event OnComponentBeginOverlap(Box)
  (params (OverlappedComponent :type Primitive%20Component%20Object%20Reference) (OtherActor :type Actor%20Object%20Reference) (OtherComp :type Primitive%20Component%20Object%20Reference) (OtherBodyIndex :type Integer) (bFromSweep :type Boolean) (SweepResult :type Hit%20Result%20Structure%20%28by%20ref%29))
  (Utilities|FlowControl|Sequence
    (:then_0
      (Audio|PlaySound2D "/Game/BluePrint/lwc/Sound/RockDookOpen.RockDookOpen"))
    (:then_1
      (bind _rockdoor (Timeline|RockMovement Play)
        (:Update
          (Transformation|SetWorldLocation (Variables|Default|GetStaticMesh) (Math|Vector|MakeVector 3.552e+04 (Math|Float|Lerp -6.4e+03 -6.84e+03 _rockdoor) -1.036e+04) false false)
          (Transformation|SetWorldLocation (Variables|Default|GetStaticMesh1) (Math|Vector|MakeVector 3.552e+04 (Math|Float|Lerp -5.4e+03 -4.95e+03 _rockdoor) -1.036e+04) false false))))))

(event OnComponentEndOverlap(Box)
  (params (OverlappedComponent :type Primitive%20Component%20Object%20Reference) (OtherActor :type Actor%20Object%20Reference) (OtherComp :type Primitive%20Component%20Object%20Reference) (OtherBodyIndex :type Integer))
  (Utilities|FlowControl|Sequence
    (:then_0
      (bind _rockdoor (Timeline|RockMovement Reverse)
        (:Update
          (Transformation|SetWorldLocation (Variables|Default|GetStaticMesh) (Math|Vector|MakeVector 3.552e+04 (Math|Float|Lerp -6.4e+03 -6.84e+03 _rockdoor) -1.036e+04) false false)
          (Transformation|SetWorldLocation (Variables|Default|GetStaticMesh1) (Math|Vector|MakeVector 3.552e+04 (Math|Float|Lerp -5.4e+03 -4.95e+03 _rockdoor) -1.036e+04) false false))))
    (:then_1
      (Audio|PlaySound2D "/Game/BluePrint/lwc/Sound/RockDookOpen.RockDookOpen"))))

(event EventBeginPlay)

(event Collision|EventActorBeginOverlap
  (params (OtherActor :type Actor%20Object%20Reference)))

(event EventTick
  (params (DeltaSeconds :type Float%20%28single-precision%29)))

(fn ConstructionScript)