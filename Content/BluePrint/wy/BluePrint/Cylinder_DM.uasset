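; Destructible cylinder that shatters when a BallPawn enters its Box and sends the player's ball to one of three preset locations.
; A random pick pairs a red, blue or yellow material with the down, up or centre location respectively.
; The chosen branch loops over the NewVar0 element indices, setting the material and applying radius damage on each pass.
; After a short delay it moves player 0's ball and destroys itself.
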(event OnComponentBeginOverlap(Box)
  (params (OverlappedComponent :type Primitive%20Component%20Object%20Reference) (OtherActor :type Actor%20Object%20Reference) (OtherComp :type Primitive%20Component%20Object%20Reference) (OtherBodyIndex :type Integer) (bFromSweep :type Boolean) (SweepResult :type Hit%20Result%20Structure%20%28by%20ref%29))
  (bind _destructible (Variables|Default|GetDestructible))
  (bind _returnvalue (Transformation|GetWorldLocation _destructible))
  (if (== (Utilities|GetClass OtherActor) "/Game/BluePrint/dgz/BallPawn.BallPawn_C")
    (switch int (Math|Random|RandomIntegerinRange 0 2)
      (:0
        (for _array_element (Variables|Default|GetNewVar_0)
          (Rendering|Material|SetMaterial _destructible _array_element "/Game/BluePrint/wy/material/red_Inst.red_Inst")
          (Class|DestructibleComponent|ApplyRadiusDamage _destructible 1e+03 _returnvalue 1e+03 1e+03 true)
          (bind _asball_pawn (Utilities|Casting|CastToBallPawn (Game|Player|GetPlayerPawn 0)))
          (Utilities|FlowControl|Delay 1.0)
          (Transformation|SetWorldLocation (Variables|/Game/BluePrint/dgz/BallPawn.BallPawn_C|GetBall _asball_pawn) (Variables|Default|GetDownLocation) false false)
          (Actor|DestroyActor)))
      (:1
        (for _array_element_2 (Variables|Default|GetNewVar_0)
          (Rendering|Material|SetMaterial _destructible _array_element_2 "/Game/BluePrint/wy/material/blue_Inst.blue_Inst")
          (Class|DestructibleComponent|ApplyRadiusDamage _destructible 1e+03 _returnvalue 1e+03 1e+03 true)
          (bind _asball_pawn_2 (Utilities|Casting|CastToBallPawn (Game|Player|GetPlayerPawn 0)))
          (Utilities|FlowControl|Delay 1.0)
          (Transformation|SetWorldLocation (Variables|/Game/BluePrint/dgz/BallPawn.BallPawn_C|GetBall _asball_pawn_2) (Variables|Default|GetUpLocation) false false)
          (Actor|DestroyActor)))
      (:2
        (for _array_element_3 (Variables|Default|GetNewVar_0)
          (Rendering|Material|SetMaterial _destructible _array_element_3 "/Game/BluePrint/wy/material/yellow_Inst.yellow_Inst")
          (Class|DestructibleComponent|ApplyRadiusDamage _destructible 1e+03 _returnvalue 1e+03 1e+03 true)
          (bind _asball_pawn_3 (Utilities|Casting|CastToBallPawn (Game|Player|GetPlayerPawn 0)))
          (Utilities|FlowControl|Delay 1.0)
          (Transformation|SetWorldLocation (Variables|/Game/BluePrint/dgz/BallPawn.BallPawn_C|GetBall _asball_pawn_3) (Variables|Default|GetCentreLocation) false false)
          (Actor|DestroyActor))))))

(event EventBeginPlay)

(event Collision|EventActorBeginOverlap
  (params (OtherActor :type Actor%20Object%20Reference)))

(event EventTick
  (params (DeltaSeconds :type Float%20%28single-precision%29)))

(fn ConstructionScript)