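; Player pawn that rolls a physics ball through the levels in VR or with a keyboard, showing the level name, a watch timer and tracking gold.
; Torque follows camera yaw, driven by an axis input or by motion-controller buttons applied on Tick, with an added offset outside third person.
; Pausing spawns a world-space menu that stays tickable, where the left controller clicks through WidgetInteraction.
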(event EventBeginPlay
  (bind _levelname (Variables|Default|GetLevelName))
  (Utilities|FlowControl|Sequence
    (:then_0
      (bind _returnvalue (Game|GetCurrentLevelName true))
      (switch string _returnvalue
        (:Map_01
          (Rendering|Components|TextRender|SetText _levelname (Variables|Default|Getl1name)))
        (:Map_02
          (Rendering|Components|TextRender|SetText _levelname (Variables|Default|Getl1name_0)))
        (:Map_03
          (Rendering|Components|TextRender|SetText _levelname (Variables|Default|Getl1name_1)))
        (:Map_07
          (Rendering|Components|TextRender|SetText _levelname (Variables|Default|Getl1name_2)))
        (:Map_05
          (Rendering|Components|TextRender|SetText _levelname (Variables|Default|Getl1name_3)))
        (:Map_6
          (Rendering|Components|TextRender|SetText _levelname (Variables|Default|Getl1name_4)))
        (:Map_Tian
          (Rendering|Components|TextRender|SetText _levelname (Variables|Default|Getl1name_5)))))
    (:then_1
      (bind _returnvalue_2 (Game|GetCurrentLevelName true))
      (if (not (Utilities|Enum|Equal(Enum) _returnvalue_2 "Map_01"))
        (bind _returnvalue_3 (Game|SpawnActorfromClass "/Game/BluePrint/dgz/所有开始iUI/m01_ui1.m01_ui1_C" (Transformation|GetWorldTransform (Variables|Default|GetFarstLocation)) "AlwaysSpawn" 0 0))
        (Variables|Default|Setb1 _returnvalue_3)))))

(event EventTick
  (params (DeltaSeconds :type Float%20%28single-precision%29))
  ;[1 1 1] 判断是否能滚
  (Utilities|FlowControl|Sequence
    (:then_0
      ;[1 1 1] 手表时间＋
      (if (Variables|Default|GetTimeBegin)
        (bind _output_get (Variables|Default|Set手表当前时间 (+ (Variables|Default|Get手表当前时间) DeltaSeconds)))
        (Rendering|Components|TextRender|SetText (Variables|Default|Getint) (Utilities|Text|ToText(Float) _output_get "HalfToEven"))))
    (:then_1
      (if (Variables|Default|GetThird%20Person)
        (if (not (Variables|Default|GetIsPause))
          (if (Variables|Default|GetIsVR)
            ;[1 1 1] 是否为按下状态
            (if (Variables|Default|GetMotionFire)
              ;[1 1 1] 球产生滚动
              (Class|PrimitiveComponent|AddTorque (Variables|Default|GetBall) (* (* (Math|Vector|GetRightVector (Math|Rotator|MakeRotator 0.0 0.0 (.Yaw (Math|Rotator|BreakRotator (Transformation|GetActorRotation (Game|GetPlayerCameraManager 0)))))) (Variables|Default|GetRunSpeed)) (Variables|Default|GetForB)) "None" false))))))
    (:then_2
      ;[1 1 1] 右手柄控小球旋转
      (if (not (Variables|Default|GetThird%20Person))
        (if (not (Variables|Default|GetIsPause))
          (if (Variables|Default|GetIsVR)
            ;[1 1 1] 是否为按下状态
            (if (Variables|Default|GetMotionFire)
              (Class|PrimitiveComponent|AddTorque (Variables|Default|GetBall) (+ (* (* (Math|Vector|GetRightVector (Math|Rotator|MakeRotator 0.0 0.0 (.Yaw (Math|Rotator|BreakRotator (Transformation|GetActorRotation (Game|GetPlayerCameraManager 0)))))) (Variables|Default|GetRunSpeed)) (Variables|Default|GetForB)) (Variables|Default|Getdsrcbabj)) "None" false))))))))

(event Input|ActionEvents|InputActionRightMotionTaked
  (params (Key :type Key%20Structure :default "AnyKey"))
  (bind _ispause (Variables|Default|GetIsPause))
  (:Pressed
    (Utilities|FlowControl|Sequence
      (:then_0
        (if (not _ispause)
          (Variables|Default|SetMotionFire true)
          (Variables|Default|SetForB 1)))))
  (:Released
    (Utilities|FlowControl|Sequence
      (:then_0
        (if (not _ispause)
          (Variables|Default|SetMotionFire false)
          (Variables|Default|SetForB 0))))))

(event Input|ActionEvents|InputActionLeftMotionTaked
  (params (Key :type Key%20Structure :default "AnyKey"))
  (bind _widgetinteraction (Variables|Default|GetWidgetInteraction))
  (bind _ispause (Variables|Default|GetIsPause))
  (:Pressed
    (Utilities|FlowControl|Sequence
      (:then_0
        (if _ispause
          ;[1 1 1] 暂停后手柄代替鼠标左键
          (Class|WidgetInteractionComponent|PressPointerKey _widgetinteraction "LeftMouseButton")
          (else
            (Variables|Default|SetMotionFire true)
            (Variables|Default|SetForB -1))))))
  (:Released
    (Utilities|FlowControl|Sequence
      (:then_0
        (if _ispause
          (Class|WidgetInteractionComponent|ReleasePointerKey _widgetinteraction "LeftMouseButton")
          (else
            (Variables|Default|SetMotionFire false)
            (Variables|Default|SetForB 0)))))))

(event Input|ActionEvents|InputActionGameStop
  (params (Key :type Key%20Structure :default "AnyKey"))
  (bind _nearlocation (Variables|Default|GetNearLocation))
  (bind _returnvalue (Transformation|GetWorldTransform _nearlocation))
  ;[1 1 1] 创建暂停
  (:Pressed
    (if (Variables|Default|GetCanPause)
      (if (Variables|Default|GetIsPause)
        (CallFunction|ResumeMyGame)
        (Variables|Default|SetCanPause true)
        (Variables|Default|SetCanWalk true)
        (Utilities|IsValid 0
          (:Is%20Valid
            (Actor|DestroyActor)))
        (else
          (bind _returnvalue_2 (Game|SpawnActorfromClass "/Game/BluePrint/dgz/Stop_widge.Stop_widge_C" (Math|Transform|MakeTransform (Math|Vector|MakeVector (.x (.location _returnvalue)) (.y (.location _returnvalue)) (.z (.location _returnvalue))) (.rotation _returnvalue) "1.000000,1.000000,1.000000") "AlwaysSpawn" 0 0))
          (bind _output_get (Variables|Default|SetWidgeActor _returnvalue_2))
          (Class|ActorComponent|SetTickablewhenPaused (Variables|/Game/BluePrint/dgz/Stop_widge.Stop_widge_C|GetWidget _output_get) true)
          (Class|ActorComponent|SetTickablewhenPaused (Variables|Default|GetBall) false)
          (Game|SetGamePaused true)
          (Variables|Default|SetIsPause true)
          (Variables|Default|SetCanPause true)
          (Variables|Default|SetCanWalk false))))))

(event Input|AxisEvents|InputAxisMoveforWorld
  (params (AxisValue :type Float%20%28single-precision%29))
  ;[1 1 1] 键盘操作
  (if (not (Variables|Default|GetIsVR))
    (Class|PrimitiveComponent|AddTorque (Variables|Default|GetBall) (* (* (Math|Vector|GetRightVector (Math|Rotator|MakeRotator 0.0 0.0 (.Yaw (Math|Rotator|BreakRotator (Transformation|GetActorRotation (Game|GetPlayerCameraManager 0)))))) (Variables|Default|GetRunSpeed)) (Math|Float|Truncate AxisValue)) "None" false)))

(fn ConstructionScript)

(fn ResumeMyGame
  (bind _widgeactor (Variables|Default|GetWidgeActor))
  (Variables|Default|SetIsPause false)
  (Utilities|IsValid _widgeactor
    (:Is%20Valid
      (Actor|DestroyActor _widgeactor)
      (Game|SetGamePaused false))))

(fn DeleteBeginWidge
  (Actor|DestroyActor)
  (Variables|Default|SetCanWalk true))

(fn AddScore
  (Variables|Default|SetGold (+ (Variables|Default|GetGold) 1)))

(fn DeleteSetting
  (Utilities|IsValid 0
    (:Is%20Valid
      (Actor|DestroyActor))))